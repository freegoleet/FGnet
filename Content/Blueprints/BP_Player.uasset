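; Player Blueprint for a networked game that shows its local net role, rocket count and health on a WBP_Role widget component.
; BeginPlay adds an FGValueReplicator named SmoothValue and writes the role text.
; Rocket and health change events update the widget through helper functions.
; Pressing B adds a random amount to the replicated value as an apparent test; the print of that value is disconnected.
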(event `self.ReceiveBeginPlay`
  (bind _returnvalue (`FGReplicatorComponent.AddReplicatorByClass` (`self.FGReplicator`) "/Script/FGNet.FGValueReplicator" "SmoothValue"))
  (bind _asfgvalue_replicator (cast `FGValueReplicator` _returnvalue))
  (set `self.ValueReplicator` _asfgvalue_replicator)
  (bind _aswbp_role (cast `/Game/Blueprints/UI/WBP_Role` (`WidgetComponent.GetUserWidgetObject` (`self.Widget_Role`))))
  (`/Game/Blueprints/UI/WBP_Role.SetLocalText` _aswbp_role (`KismetTextLibrary.Conv_StringToText` (`|GetEnumeratorNameAsString` (`self.GetLocalRole`)))))

(event `self.ReceiveTick`
  (params (DeltaSeconds :type "Float (single-precision)")))

(event `Key|B`
  (params (Key :type "Key Structure"))
  (:`Pressed`
    (`FGValueReplicator.SetValue` (`self.ValueReplicator`) (+ (`FGValueReplicator.GetValue` (`self.ValueReplicator`)) (`KismetMathLibrary.RandomFloatInRange` 10.0 200.0)))))

(event `self.BP_OnNumRocketsChanged`
  (params (NewNumRockets :type Integer))
  (`self.SetNumRocketsInWidget` NewNumRockets))

(event `self.BP_OnPlayerHealthChanged`
  (params (NewPlayerHealth :type Integer))
  (`self.SetPlayerHealthInWidget` NewPlayerHealth))

(fn `SetNumRocketsInWidget`
  (params (InNumRockets :type Integer))
  (bind _aswbp_role (cast `/Game/Blueprints/UI/WBP_Role` (`WidgetComponent.GetUserWidgetObject` (`self.Widget_Role`))))
  (`/Game/Blueprints/UI/WBP_Role.SetNumRockets` _aswbp_role InNumRockets))

(fn `SetPlayerHealthInWidget`
  (params (InPlayerHealth :type Integer))
  (bind _aswbp_role (cast `/Game/Blueprints/UI/WBP_Role` (`WidgetComponent.GetUserWidgetObject` (`self.Widget_Role`))))
  (`/Game/Blueprints/UI/WBP_Role.SetPlayerHealth` _aswbp_role InPlayerHealth))

(fn `UserConstructionScript`)